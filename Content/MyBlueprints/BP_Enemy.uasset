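; BP_Enemy is an enemy actor with an Hp value that is reduced by damage.
; AnyDamage and skeletal mesh hit events share one chain that subtracts the AnyDamage event's Damage output from Hp, even when a hit triggers it.
; At zero Hp or below, it prints Hp and destroys the hit event's OtherActor rather than itself.
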(event `self.ReceiveAnyDamage`
  (params (Damage :type "Float (single-precision)") (DamageType :type "DamageType Object Reference") (InstigatedBy :type "Controller Object Reference") (DamageCauser :type "Actor Object Reference"))
  (bind _output_get (set `self.Hp` (- (`self.Hp`) Damage) :!label _label))
  (if (<= _output_get 0.0)
    (`KismetSystemLibrary.PrintString` (`KismetStringLibrary.Conv_DoubleToString` _output_get))
    (`self.K2_DestroyActor` (stale `self.SkeletalMesh.OnComponentHit` OtherActor))))

(event `self.SkeletalMesh.OnComponentHit`
  (params (HitComponent :type "PrimitiveComponent Object Reference") (OtherActor :type "Actor Object Reference") (OtherComp :type "PrimitiveComponent Object Reference") (NormalImpulse :type "Vector Structure") (Hit :type "HitResult Structure (by ref)"))
  (goto _label))

(fn `UserConstructionScript`)